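; BP_Objeto deforms a copy of a static mesh with Perlin noise using Geometry Script.
; The construction script copies the mesh and applies PN tessellation to add vertices for displacement.
; BeginPlay applies noise driven by Magnitude, Frequency and Seed, then recomputes normals.
; The construction script also creates a dynamic material instance, but the nodes that store and assign it to Ball never run.
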(event `self.ReceiveBeginPlay`
  (bind _returnvalue (`GeometryScriptLibrary_MeshDeformFunctions.ApplyPerlinNoiseToMesh` null (struct) (make `GeometryScriptPerlinNoiseOptions` (make `GeometryScriptPerlinNoiseLayerOptions` (`self.Magnitude`) (`self.Frequency`) (0.0 0.0 0.0) (`self.Seed`))) null))
  (`GeometryScriptLibrary_MeshNormalsFunctions.RecomputeNormals` _returnvalue (struct) false null))

(fn `UserConstructionScript`
  (`GeometryScriptLibrary_StaticMeshFunctions.CopyMeshFromStaticMesh` null null (struct) (struct) null
    (:`Success`
      (bind _returnvalue (`KismetMaterialLibrary.CreateDynamicMaterialInstance` "/Engine/EngineMaterials/DefaultDeferredDecalMaterial.DefaultDeferredDecalMaterial" "None"))
      (`GeometryScriptLibrary_MeshSubdivideFunctions.ApplyPNTessellation` null (struct) 6 null))))