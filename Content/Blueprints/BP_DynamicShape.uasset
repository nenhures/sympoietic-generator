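; BP_DynamicShape is a Geometry Script generated mesh actor that builds a noise-displaced shape from a source static mesh.
; On each rebuild it copies SourceMesh into the dynamic mesh, applies PN tessellation, displaces it with seeded Perlin noise and recomputes normals.
; Magnitude, Frequency and Seed drive the noise, the resulting mesh is stored in NewMesh, and GetDynamicMeshRef returns the actor itself.
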(event `self.OnRebuildGeneratedMesh`
  (params (TargetMesh :type "DynamicMesh Object Reference"))
  (bind _sourcemesh (`self.SourceMesh`)
    (:`then`
      (bind _returnvalue (`GeometryScriptLibrary_StaticMeshFunctions.CopyMeshFromStaticMesh` _sourcemesh TargetMesh (struct) (struct) null)
        (:`Success`
          (bind _returnvalue_2 (`GeometryScriptLibrary_MeshSubdivideFunctions.ApplyPNTessellation` _returnvalue (struct) 6 null))
          (bind _returnvalue_3 (`GeometryScriptLibrary_MeshDeformFunctions.ApplyPerlinNoiseToMesh` _returnvalue_2 (struct) (make `GeometryScriptPerlinNoiseOptions` (make `GeometryScriptPerlinNoiseLayerOptions` (`self.Magnitude`) (`self.Frequency`) (0.0 0.0 0.0) (`self.Seed`))) null))
          (bind _returnvalue_4 (`GeometryScriptLibrary_MeshNormalsFunctions.RecomputeNormals` _returnvalue_3 (struct) false null))
          (set `self.NewMesh` _returnvalue_4))))
    (:`else`)))

(fn `GetDynamicMeshRef`
  (returns (GeneratedMesh :type "/Game/Blueprints/BP_DynamicShape Object Reference"))
  (return self))

(fn `UserConstructionScript`)